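; AI controller for guard NPCs that patrol and react to sensed actors.
; On BeginPlay it loads the patrol blackboard and runs the guard behavior tree.
; AI perception updates write actors lacking the enemy tag to the blackboard's enemy key on successful sensing and clear it when sensing fails.
; A player-position polling timer, debug printing and hardcoded patrol points remain as disconnected leftovers.
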(event OnTargetPerceptionUpdated(AIPerception)
  (params (Actor :type Actor%20Object%20Reference) (Stimulus :type AI%20Stimulus%20Structure))
  ;[1 1 1] Sense Enemy
  (if (not (Actor|ActorHasTag Actor (Variables|Default|GetEnemyTag)))
    (if (.bSuccessfullySensed (Utilities|Struct|BreakAIStimulus Stimulus))
      (AI|Components|Blackboard|SetValueasObject (Variables|Default|GetBlackboardComponent) (Variables|Default|GetEnemyKey) Actor)
      (else
        (AI|Components|Blackboard|ClearValue (Variables|Default|GetBlackboardComponent) (Variables|Default|GetEnemyKey))))))

(event Custom|UpdatePlayerPosition
  ;[1 1 1] SetEnemyPosition
  (AI|Components|Blackboard|SetValueasObject (Variables|Default|GetBlackboardComponent) (Variables|Default|GetEnemyKey) (Game|Player|GetPlayerPawn 0)))

(event EventBeginPlay
  ;[1 1 1] SetBlackboardAndBehaviourTree
  (bind _blackboardcomponent (Class|AIController|UseBlackboard "/Game/Dynamic/NPC/AI/BB_PatrolData.BB_PatrolData"))
  (Variables|Default|SetBlackboardComponent _blackboardcomponent)
  (AI|RunBehaviorTree "/Game/Dynamic/NPC/AI/BT_GuardBehaviour.BT_GuardBehaviour"))

(fn ConstructionScript)