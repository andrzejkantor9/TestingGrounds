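; AI controller for a patrolling guard, driving its BP_Character through the BT_GuardBehaviour behavior tree and BB_PatrolData blackboard.
; AI perception writes sensed actors lacking the enemy tag to the blackboard's enemy key, and clears it when sensing fails so the guard turns suspicious.
; A looping timer meant for aim and shoot animation flags calls an empty event; that flag logic and older debug code are disconnected.
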(event OnTargetPerceptionUpdated(AIPerception)
  (params (Actor :type Actor%20Object%20Reference) (Stimulus :type AI%20Stimulus%20Structure))
  ;[1 1 1] Sense Enemy
  ;;[1 1 1] Isn't AI
  (if (not (Actor|ActorHasTag Actor (Variables|Default|GetEnemyTag)))
    (if (.bSuccessfullySensed (Utilities|Struct|BreakAIStimulus Stimulus))
      ;;[1 1 1] Follow Enemy
      (AI|Components|Blackboard|SetValueasObject (Variables|Default|GetBlackboardComponent) (Variables|Default|GetEnemyKey) Actor)
      (else
        ;;[1 1 1] Go to suspicious state
        (AI|Components|Blackboard|ClearValue (Variables|Default|GetBlackboardComponent) (Variables|Default|GetEnemyKey))))))

(event Custom|0,1Tick
  ;[1 1 1] Update Shooting and Aiming Animation Flags
)

(event EventBeginPlay
  ;[1 1 1] Set Blackboard And BehaviourTree
  (bind _blackboardcomponent (Class|AIController|UseBlackboard "/Game/Dynamic/Characters/AI/BB_PatrolData.BB_PatrolData"))
  (Variables|Default|SetBlackboardComponent _blackboardcomponent)
  (AI|RunBehaviorTree "/Game/Dynamic/Characters/AI/BT_GuardBehaviour.BT_GuardBehaviour")
  ;[1 1 1] Cache BP_Character
  (bind _asbp_character (Utilities|Casting|CastToBP_Character (Pawn|GetControlledPawn)))
  (Variables|Default|SetBP_Character _asbp_character)
  ;[1 1 1] Update Shooting and Aiming Animation Flags
  (Utilities|Time|SetTimerbyEvent (delegate Custom|0,1Tick) 0.1 true))

(fn ConstructionScript)