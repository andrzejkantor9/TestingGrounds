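; BP_FireComponent is a weapon behaviour component that fires a projectile for a character.
; Its Fire function spawns BP_FirstPersonProjectile at the component's own world transform, with the passed-in character as owner.
; BeginPlay and Tick are empty.
; Disconnected leftover nodes would report a noise event and pick the first- or third-person gun by display name, but none of them run.
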(event EventBeginPlay)

(event EventTick
  (params (DeltaSeconds :type Float%20%28single-precision%29)))

(fn Fire
  (params (Character :type BP%20Character%20Object%20Reference))
  (Game|SpawnActorfromClass "/Game/Dynamic/Weapons/Behaviour/BP_FirstPersonProjectile.BP_FirstPersonProjectile_C" (Transformation|GetWorldTransform) "Undefined" Character 0))