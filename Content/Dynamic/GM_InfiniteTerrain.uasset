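; Game mode for an infinite terrain that spawns and retires tiles as a chain.
; BeginPlay spawns three tiles, each placed at the previous tile's attach location, and unlocks the first when UnlockFirstTile is set.
; ProceedDestroyTile destroys the previously stored tile and stores the one passed in, so removal lags one tile behind.
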(event EventBeginPlay
  (for _index (range 0 2)
    (CallFunction|SpawnTile)))

(fn ConstructionScript)

(fn SpawnTile
  (bind _returnvalue (Game|SpawnActorfromClass "/Game/Dynamic/Levels/Tile.Tile_C" (Variables|Default|GetTileSpawnTransform) "Undefined" 0 0))
  (bind _attachtransform (Default|GetAttachLocation _returnvalue))
  (Variables|Default|SetTileSpawnTransform _attachtransform)
  (if (Variables|Default|GetUnlockFirstTile)
    (Default|LockTile _returnvalue false)
    (Variables|Default|SetUnlockFirstTile false)))

(fn ProceedDestroyTile
  (params (TileToDestroyNext :type Tile%20Object%20Reference))
  (if (Utilities|IsValid (Variables|Default|GetTileToDestroy))
    (Actor|DestroyActor (Variables|Default|GetTileToDestroy)))
  (Variables|Default|SetTileToDestroy TileToDestroyNext))