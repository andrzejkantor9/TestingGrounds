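; Level tile for infinite terrain that scatters props and AI characters across itself on BeginPlay.
; Its gate starts locked (red, collidable) and opens green while the player is inside the locking volume.
; When the player leaves that volume, the gate relocks and the tile asks GM_InfiniteTerrain to spawn another tile and proceed with destroying this one.
; GetAttachLocation exposes the Arrow's world transform as an attach point.
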(event OnComponentEndOverlap(LockingVloume)
  (params (OverlappedComponent :type Primitive%20Component%20Object%20Reference) (OtherActor :type Actor%20Object%20Reference) (OtherComp :type Primitive%20Component%20Object%20Reference) (OtherBodyIndex :type Integer))
  (if (== OtherActor (Game|GetPlayerCharacter 0))
    (CallFunction|LockTile true)
    (bind _asgm_infinite_terrain (Utilities|Casting|CastToGM_InfiniteTerrain (Game|GetGameMode)))
    (Default|SpawnTile _asgm_infinite_terrain)
    ;[1 1 1] TODO despawn static meshes
    (Default|ProceedDestroyTile _asgm_infinite_terrain self)))

(event OnComponentBeginOverlap(LockingVloume)
  (params (OverlappedComponent :type Primitive%20Component%20Object%20Reference) (OtherActor :type Actor%20Object%20Reference) (OtherComp :type Primitive%20Component%20Object%20Reference) (OtherBodyIndex :type Integer) (bFromSweep :type Boolean) (SweepResult :type Hit%20Result%20Structure%20%28by%20ref%29))
  ;[1 1 1] ForProperObjectSpawning
  (CallFunction|UnlockGateonBeginOverlap OtherActor))

(event EventBeginPlay
  (CallFunction|LockTile true)
  ;[1 1 1] TODO make cannisters not spawn on green wall
  (Class|Tile|PlaceActors "/Game/Dynamic/Levels/Props/BP_Container.BP_Container_C" 0 4 4.5e+02 1.0 1.0)
  (Class|Tile|PlaceActors "/Game/Dynamic/Levels/Props/BP_Box.BP_Box_C" 1 4 125.0 1.0 4.0)
  (Class|Tile|PlaceActors "/Game/Dynamic/Levels/Props/BP_Canister.BP_Canister_C" 2 7 8e+01 1.0 2.0)
  (Class|Tile|PlaceActors "/Game/Dynamic/Levels/Props/BP_SandbagWall.BP_SandbagWall_C" 1 2 2.5e+02 1.0 1.0)
  (Class|Tile|PlaceActors "/Game/Dynamic/Levels/Props/BP_Rock01.BP_Rock01_C" 0 4 1.5e+02 1.0 4.0)
  (Class|Tile|PlaceActors "/Game/Dynamic/Levels/Props/BP_Rock05.BP_Rock05_C" 1 2 2.5e+02 1.0 4.0)
  (Class|Tile|PlaceActors "/Game/Dynamic/Levels/Props/BP_Rock05.BP_Rock05_C" 0 2 2.5e+02 1.0 4.0)
  (Class|Tile|PlaceActors "/Game/Dynamic/Levels/Props/BP_Rock17.BP_Rock17_C" 1 2 2.5e+02 1.0 4.0)
  (Class|Tile|PlaceActors "/Game/Dynamic/Levels/Props/BP_Rock17.BP_Rock17_C" 0 2 2.5e+02 1.0 4.0)
  (Class|Tile|PlaceAIPawns "/Game/Dynamic/Characters/Behaviour/BP_Character.BP_Character_C" 2 4 5e+02))

(fn ConstructionScript)

(fn GetAttachLocation
  (return (Transformation|GetWorldTransform (Variables|Default|GetArrow))))

(fn LockTile
  (params (Lock :type Boolean))
  (Collision|SetCollisionEnabled (Variables|Default|GetGate) (select Lock "QueryAndPhysics" "NoCollision"))
  (Rendering|Material|SetMaterial (Variables|Default|GetGate) 0 (select Lock "/Game/Dynamic/Levels/MI_Barrier_Red.MI_Barrier_Red" "/Game/Dynamic/Levels/MI_Barrier_Green.MI_Barrier_Green")))

(fn UnlockGateonBeginOverlap
  (params (OverlappingActor :type Actor%20Object%20Reference))
  (if (== OverlappingActor (Game|GetPlayerCharacter 0))
    (CallFunction|LockTile false)))