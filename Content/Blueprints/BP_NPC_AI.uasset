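; NPC AI controller that starts patrol behavior for the pawn it controls.
; On BeginPlay it initializes the PatrolData blackboard and runs the Patrol behavior tree.
; A FindPatrolPoint function writes the first entry of the controlled ThirdPersonCharacter's PatrolPoints array to the Waypoint key, but its only call here is disconnected.
; Disconnected nodes also hold hard-coded WorldOrigin and PatrolPoint vector writes that never run.
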(event EventBeginPlay
  (Class|AIController|UseBlackboard "/Game/Blueprints/PatrolData.PatrolData")
  (AI|RunBehaviorTree "/Game/Blueprints/Patrol.Patrol"))

(fn ConstructionScript)

(fn FindPatrolPoint
  (params (BlackboardComponent :type Blackboard%20Component%20Object%20Reference))
  (bind _asthird_person_character (Utilities|Casting|CastToThirdPersonCharacter (Pawn|GetControlledPawn)))
  (AI|Components|Blackboard|SetValueasObject BlackboardComponent (Utilities|Name|MakeLiteralName "Waypoint") (Utilities|Array|Get(acopy) (Variables|/Game/ThirdPersonCPP/Blueprints/ThirdPersonCharacter.ThirdPersonCharacter_C|GetPatrolPoints _asthird_person_character))))