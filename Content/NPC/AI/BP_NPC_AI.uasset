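; AI controller for patrolling NPCs that starts the PatrolData blackboard and runs the BT_Patrol behavior tree on BeginPlay.
; AI Perception updates only print the pawn, the encountered actor and the sense used.
; FindPatrolPoint, which stores the ThirdPersonCharacter pawn's first patrol point as the Waypoint key, sits on a disconnected branch.
; The nodes setting WorldOrigin and PatrolPoint vector keys are also disconnected.
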(event OnTargetPerceptionUpdated(AIPerception)
  (params (Actor :type Actor%20Object%20Reference) (Stimulus :type AI%20Stimulus%20Structure))
  (bind _returnvalue (Class|AIPerceptionSystem|GetSenseClassforStimulus Stimulus))
  (Development|PrintString (Utilities|String|Append (Utilities|GetDisplayName (Pawn|GetControlledPawn)) " has ecountered " (Utilities|GetDisplayName Actor) " using: " (Utilities|GetClassDisplayName _returnvalue))))

(event EventBeginPlay
  (Class|AIController|UseBlackboard "/Game/NPC/AI/PatrolData.PatrolData")
  (AI|RunBehaviorTree "/Game/NPC/AI/BT_Patrol.BT_Patrol"))

(fn ConstructionScript)

(fn FindPatrolPoint
  (params (BlackboardComponent :type Blackboard%20Component%20Object%20Reference))
  (bind _asthird_person_character (Utilities|Casting|CastToThirdPersonCharacter (Pawn|GetControlledPawn)))
  (AI|Components|Blackboard|SetValueasObject BlackboardComponent (Utilities|Name|MakeLiteralName "Waypoint") (Utilities|Array|Get(acopy) (Variables|/Game/zzzTrash/ThirdPersonCharacter.ThirdPersonCharacter_C|GetPatrolPoints_0 _asthird_person_character))))